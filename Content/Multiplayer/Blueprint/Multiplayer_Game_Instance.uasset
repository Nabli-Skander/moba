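; Game instance for multiplayer that handles hosting, finding, joining and invites through Advanced Sessions nodes, plus the related menu widgets.
; Session creation stores name, map and game mode as extra settings, then always opens ThirdPersonExampleMap as a listen server, whatever map is passed.
; Searches cache results and refresh the passed server list widget.
; List and creation widgets are created once and reused, while each received invite spawns a new popup.
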(event `Join`
  (params (Session :type "BlueprintSessionResult Structure"))
  ;[1 1 1] join
  (`JoinSessionCallbackProxy.JoinSession` (`GameplayStatics.GetPlayerController` 0) Session))

(event `Create session`
  (params (Nom :type String) (Map :type String) (`Game Mode` :type String) (PublicConnections :type Integer) (bUseLAN :type Boolean))
  ;[1 1 1] create session
  (`CreateSessionCallbackProxyAdvanced.CreateAdvancedSession` (`|MakeArray` (`AdvancedSessionsLibrary.MakeLiteralSessionPropertyString` "Nom" Nom) (`AdvancedSessionsLibrary.MakeLiteralSessionPropertyString` "Map" Map) (`AdvancedSessionsLibrary.MakeLiteralSessionPropertyString` "Gamemode" `Game Mode`)) (`GameplayStatics.GetPlayerController` 0) PublicConnections 0 bUseLAN
    (:`OnSuccess`
      (`GameplayStatics.OpenLevel` "ThirdPersonExampleMap" true "listen"))))

(event `show server list`
  (bind _returnvalue (`GameplayStatics.GetPlayerController` 0))
  ;[1 1 1] show server list
  (`/Engine/EditorBlueprintResources/StandardMacros.IsValid` (`self.server list`)
    (:`Is Valid`
      (`UserWidget.AddToViewport` (`self.server list`) 0))
    (:`Is Not Valid`
      (bind _returnvalue_2 (`|CreateWidget` "/Game/Multiplayer/Hud/Server_List.Server_List_C" _returnvalue))
      (bind _output_get (set `self.server list` _returnvalue_2))
      (`UserWidget.AddToViewport` _output_get 0)
      (set `PlayerController.bShowMouseCursor` true _returnvalue))))

(event `show server_create`
  (bind _returnvalue (`GameplayStatics.GetPlayerController` 0))
  ;[1 1 1] show server create
  (`/Engine/EditorBlueprintResources/StandardMacros.IsValid` (`self.server create`)
    (:`Is Valid`
      (`UserWidget.AddToViewport` (`self.server create`) 0))
    (:`Is Not Valid`
      (bind _returnvalue_2 (`|CreateWidget` "/Game/Multiplayer/Hud/Server_Create.Server_Create_C" _returnvalue))
      (bind _output_get (set `self.server create` _returnvalue_2))
      (`UserWidget.AddToViewport` _output_get 0)
      (set `PlayerController.bShowMouseCursor` true _returnvalue))))

(event `find session`
  (params (`sever list` :type "/Game/Multiplayer/Hud/Server_List Object Reference"))
  ;[1 1 1] Find Session
  (`KismetArrayLibrary.Array_Clear` (`self.FoundSessions`))
  (bind _results (`FindSessionsCallbackProxyAdvanced.FindSessionsAdvanced` (`GameplayStatics.GetPlayerController` 0) 0 false "AllServers")
    (:`OnSuccess`
      (set `self.FoundSessions` _results)
      (set `/Game/Multiplayer/Hud/Server_List.Found Session` _results `sever list`)
      (`/Game/Multiplayer/Hud/Server_List.Update Server list` `sever list`))))

(event `self.OnSessionInviteReceived`
  (params (LocalPlayerNum :type Integer) (PersonInviting :type "BPUniqueNetId Structure") (AppId :type String) (SessionToJoin :type "BlueprintSessionResult Structure (by ref)"))
  ;[1 1 1] Invite
  (bind _returnvalue (`|CreateWidget` "/Game/Multiplayer/Hud/Invite.Invite_C" (`GameplayStatics.GetPlayerController` 0) SessionToJoin PersonInviting))
  (`UserWidget.AddToViewport` _returnvalue 0))